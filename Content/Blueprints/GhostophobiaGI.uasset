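; Ghostophobia's game instance, judging by its name, handling lobby session creation, widget display and camera post-process changes.
; CreateLobby hosts an Advanced Sessions session named with a generated GUID, then opens the Lobby level on success.
; Widget requests pass through wrapper events that add widgets to the viewport and set mouse visibility.
; An init event caches the player character for camera changes, while UpdateEmfLevel is a stub returning zero.
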(event Custom|Create%20Lobby
  (params (Players :type Integer))
  ;[1 1 1] Create Lobby
  (Variables|Session|SetServer%20Name (Session|GenerateSessionName))
  (bind _output_get (Variables|Session|SetMax%20Connections Players))
  (|AdvancedSession (Utilities|Array|MakeArray (Class|AdvancedSessionsLibrary|MakeLiteralSessionPropertyString "SessionName" (Session|GenerateSessionName))) (Game|GetPlayerController 0) _output_get 0 false true false true true true false false false true
    (:OnSuccess
      (Game|OpenLevel(byObjectReference) "/Game/GhostophobiaBP/Maps/Lobby.Lobby" true "Listen"))))

(event Custom|Create%20Widget%20On%20One%20Screen
  (params (Class :type User%20Widget%20Class%20Reference) (Show%20Mouse%20Cursor :type Boolean))
  ;[1 1 1] Create Widget On 1 Screen
  (CallFunction|CreateWidgetClient1Screen Class Show%20Mouse%20Cursor))

(event Custom|Create%20Widget%20Client%201%20Screen
  (params (Class :type User%20Widget%20Class%20Reference) (Show%20Mouse%20Cursor :type Boolean))
  ;[1 1 1] Create Widget On 1 Screen
  (bind _returnvalue (UserInterface|CreateWidget Class))
  (UserInterface|Viewport|AddtoViewport _returnvalue 0)
  (Variables|/Script/Engine.PlayerController|SetbShowMouseCursor (Game|GetPlayerController 0) Show%20Mouse%20Cursor))

(event Custom|Widget%20For%20All
  (params (Class :type User%20Widget%20Class%20Reference) (Mouse :type Boolean))
  ;[1 1 1] Widget For All
  (bind _returnvalue (UserInterface|CreateWidget Class))
  (UserInterface|Viewport|AddtoViewport _returnvalue 0)
  (Variables|/Script/Engine.PlayerController|SetbShowMouseCursor (Game|GetPlayerController 0) Mouse))

(event Custom|INt
  (bind _asghostophobia_character (Utilities|Casting|CastToGhostophobiaCharacter (Game|GetPlayerCharacter 0)))
  (Variables|Default|SetCharacter _asghostophobia_character))

(event EventWidgetonOneScreen
  (params (Widget :type User%20Widget%20Class%20Reference) (Mouse :type Boolean))
  ;[1 1 1] Create Widget On 1 Screen
  (CallFunction|CreateWidgetonOneScreen Widget Mouse))

(event EventCreateWidgetforAll
  (params (Widget :type User%20Widget%20Class%20Reference) (Mouse :type Boolean))
  ;[1 1 1] Widget For All
  (CallFunction|WidgetforAll Widget Mouse))

(event EventChangePostProccesCamera
  (params (NewParam :type Post%20Process%20Settings%20Structure))
  (Default|ChangeCamera (Variables|Default|GetCharacter) NewParam))

(fn GenerateSessionName
  (return (Guid|ToString(Guid) (Guid|NewGuid))))

(fn UpdateEmfLevel
  (params (Level :type Integer))
  (return 0))