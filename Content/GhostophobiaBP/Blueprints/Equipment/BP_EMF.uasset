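; EMF reader equipment for Ghostophobia that the player picks up through an Interact prompt.
; Interact calls the character's weapon check and server pickup, while target events forward to the child-actor prompt widget configured by Set* overrides.
; UpdateEmfLevel maps levels to a green, yellow or red spotlight.
; The two red levels start the EMF sound; lower levels request it off, but PlayEMFAudioClient ignores false, so that path never stops it.
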(event Custom|Play%20EMF%20Audio
  (params (Enable :type Boolean))
  (CallFunction|PlayEMFAudioClient Enable))

(event Custom|Play%20EMF%20Audio%20Client
  (params (Enable :type Boolean))
  (if (Variables|Default|GetEnable)
    (CallFunction|AudioEMF Enable)))

(event EventCurrentTarget
  (params (Pawn :type Pawn%20Object%20Reference))
  (bind _widget (Variables|Default|GetWidget))
  (bind _childactor (Variables|/Script/Engine.ChildActorComponent|GetChildActor _widget))
  ;[1 1 1] Current target (Copy and paste this in to your own actor)
  (Class|InteractionInterface|CurrentTarget(Message) _childactor Pawn)
  (Class|InteractionInterface|ParentActor(Message) _childactor self))

(event EventClearTarget
  ;[1 1 1] Clear target (Copy and paste this in to your own actor)
  (Class|InteractionInterface|ClearTarget(Message) (Variables|/Script/Engine.ChildActorComponent|GetChildActor (Variables|Default|GetWidget))))

(event EventBeginPlay
  (bind _asghostophobia_character (Utilities|Casting|CastToGhostophobiaCharacter (Game|GetPlayerCharacter 0)))
  (Variables|Default|SetChar%20Ref _asghostophobia_character))

(event EventInteract
  (params (Key :type Key%20Structure) (Pawn :type Pawn%20Object%20Reference))
  ;[1 1 1] Print screen the key the player interacted with
  (bind _asghostophobia_character (Utilities|Casting|CastToGhostophobiaCharacter Pawn))
  (Default|CheckandTakeWeapon (Variables|/Game/GhostophobiaBP/Character/Blueprints/GhostophobiaCharacter.GhostophobiaCharacter_C|GetWeapon _asghostophobia_character) "NewEnumerator4")
  (Default|PickUpWeaponServer _asghostophobia_character self))

(fn ConstructionScript
  (|CallParentFunction))

(fn SwitchColorLight
  (params (Selection :type Integer))
  (switch int Selection
    (:1
      (Utilities|SetLightColor "(R=0.000000,G=1.000000,B=0.137072,A=1.000000)")
      (CallFunction|PlayEMFAudio false))
    (:2
      (Utilities|SetLightColor "(R=0.000000,G=1.000000,B=0.137072,A=1.000000)")
      (CallFunction|PlayEMFAudio false))
    (:3
      (Utilities|SetLightColor "(R=1.000000,G=0.867299,B=0.000000,A=1.000000)")
      (CallFunction|PlayEMFAudio false))
    (:4
      (Utilities|SetLightColor "(R=1.000000,G=0.000000,B=0.041492,A=1.000000)")
      (CallFunction|PlayEMFAudio true))
    (:5
      (Utilities|SetLightColor "(R=1.000000,G=0.000000,B=0.041492,A=1.000000)")
      (CallFunction|PlayEMFAudio true))))

(fn AudioEMF
  (params (Enable :type Boolean))
  (bind _emf_sound (Variables|Default|GetEMF_Sound))
  (if Enable
    (Audio|Components|Audio|Play _emf_sound 0.0)
    (else
      (Audio|Components|Audio|Stop _emf_sound))))

(fn SetDetail1
  (return false ""))

(fn SetDetail2
  (return false ""))

(fn SetDetail3
  (return false ""))

(fn SetDetail4
  (return false ""))

(fn SetWidgetAmount
  (return false 0))

(fn SetWidgetColor
  (return "" ""))

(fn SetWidgetKeyBinds
  (return true (Utilities|Array|MakeArray (Utilities|Struct|MakeS_KeyBinds "E" "Interact"))))

(fn SetWidgetLevel
  (return false ""))

(fn SetWidgetSubTitle
  (return false ""))

(fn SetWidgetTitle
  (return true "Interact"))

(fn SetWidgetType
  (return "NewEnumerator1"))

(fn UpdateEmfLevel
  (params (Level :type Integer))
  (CallFunction|SwitchColorLight Level)
  (return 0))