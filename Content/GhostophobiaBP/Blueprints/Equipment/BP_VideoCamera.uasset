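; BP_VideoCamera is an interactable video camera equipment actor.
; On Interact it calls the player character's weapon CheckAndTakeWeap with an enum slot, then passes itself to InteractVDCamera.
; Target and clear-target events relay to a child-actor prompt widget, configured by Set Widget functions with an "Interact" title and E key bind.
; BeginPlay caches the player character, though nothing here reads it.
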(event EventBeginPlay
  (Variables|Default|SetChar (.AsGhostophobia%20Character (Utilities|Casting|CastToGhostophobiaCharacter (Game|GetPlayerCharacter 0)))))

(event EventCurrentTarget
  (params (Pawn :type Pawn%20Object%20Reference))
  (bind _widget (Variables|Default|GetWidget))
  (bind _childactor (Variables|/Script/Engine.ChildActorComponent|GetChildActor _widget))
  ;[1 1 1] Current target (Copy and paste this in to your own actor)
  (Class|InteractionInterface|CurrentTarget(Message) _childactor Pawn)
  (Class|InteractionInterface|ParentActor(Message) _childactor self))

(event EventClearTarget
  ;[1 1 1] Clear target (Copy and paste this in to your own actor)
  (Class|InteractionInterface|ClearTarget(Message) (Variables|/Script/Engine.ChildActorComponent|GetChildActor (Variables|Default|GetWidget))))

(event EventInteract
  (params (Key :type Key%20Structure :default "None") (Pawn :type Pawn%20Object%20Reference))
  ;[1 1 1] Print screen the key the player interacted with
  (bind _asghostophobia_character (Utilities|Casting|CastToGhostophobiaCharacter Pawn))
  (Default|CheckandTakeWeap (Variables|/Game/GhostophobiaBP/Character/Blueprints/GhostophobiaCharacter.GhostophobiaCharacter_C|GetWeapon _asghostophobia_character) "NewEnumerator3")
  (Default|InteractVDCamera _asghostophobia_character self))

(fn ConstructionScript)

(fn SetDetail1
  (return false ""))

(fn SetDetail2
  (return false ""))

(fn SetDetail3
  (return false ""))

(fn SetDetail4
  (return false ""))

(fn SetWidgetAmount
  (return false 0))

(fn SetWidgetColor
  (return "" ""))

(fn SetWidgetKeyBinds
  (return true (Utilities|Array|MakeArray (Utilities|Struct|MakeS_KeyBinds "E" "Interact"))))

(fn SetWidgetLevel
  (return false ""))

(fn SetWidgetSubTitle
  (return false ""))

(fn SetWidgetTitle
  (return true "Interact"))

(fn SetWidgetType
  (return "NewEnumerator1"))