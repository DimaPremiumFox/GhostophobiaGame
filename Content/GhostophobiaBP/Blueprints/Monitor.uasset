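; Interactable monitor actor that shows a "Main Menu" prompt with an "Open Lobby" key bind on E.
; On interact, it asks the GhostophobiaGI game instance to put its configured widget class on screen with mouse enabled.
; Target and clear-target events forward to the prompt's child actor, whose content comes from the SetWidget and SetDetail overrides.
; A BeginPlay timeline animates the text render's height.
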(event EventBeginPlay
  (bind _asghostophobia_character (Utilities|Casting|CastToGhostophobiaCharacter (Game|GetPlayerCharacter 0)))
  (Variables|Default|SetChar _asghostophobia_character)
  (bind _text (Timeline|Text Play)
    (:Update
      (Transformation|SetRelativeLocation (Variables|Default|GetTextRender) (Math|Vector|MakeVector -19.999994 -6.9e-05 _text) false false))))

(event EventCurrentTarget
  (params (Pawn :type Pawn%20Object%20Reference))
  (bind _widget (Variables|Default|GetWidget))
  (bind _childactor (Variables|/Script/Engine.ChildActorComponent|GetChildActor _widget))
  ;[1 1 1] Current target (Copy and paste this in to your own actor)
  (Class|InteractionInterface|CurrentTarget(Message) _childactor Pawn)
  (Class|InteractionInterface|ParentActor(Message) _childactor self))

(event EventClearTarget
  ;[1 1 1] Clear target (Copy and paste this in to your own actor)
  (Class|InteractionInterface|ClearTarget(Message) (Variables|/Script/Engine.ChildActorComponent|GetChildActor (Variables|Default|GetWidget))))

(event EventInteract
  (params (Key :type Key%20Structure) (Pawn :type Pawn%20Object%20Reference))
  ;[1 1 1] Print screen the key the player interacted with
  (Class|Multiplayer|WidgetonOneScreen(Message) (.AsGhostophobia%20GI (Utilities|Casting|CastToGhostophobiaGI (Game|GetGameInstance))) (Variables|Default|GetClassWidget) true))

(fn ConstructionScript)

(fn SetDetail1
  (return false ""))

(fn SetDetail2
  (return false ""))

(fn SetDetail3
  (return false ""))

(fn SetDetail4
  (return false ""))

(fn SetWidgetAmount
  (return false 0))

(fn SetWidgetColor
  (bind (_return_value _dark_color _light_color) (CallFunction|GetQualityColor (Utilities|Struct|MakeDataTableRowHandle "/Game/InteractionWidgets/Blueprints/QualitysColors.QualitysColors" "Junk")))
  (return _dark_color _light_color))

(fn SetWidgetKeyBinds
  (return true (Utilities|Array|MakeArray (Utilities|Struct|MakeS_KeyBinds "E" "Open Lobby"))))

(fn SetWidgetLevel
  (return false ""))

(fn SetWidgetSubTitle
  (return false ""))

(fn SetWidgetTitle
  (return true "Main Menu"))

(fn SetWidgetType
  (return "NewEnumerator0"))