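; Haunted house actor that drives ghost activity while a player character is inside its Box, with the ghost type set on the authority.
; Overlap starts a looping GhostEvents timer, with interval and activity threshold set per ghost type in the construction script.
; Each tick may throw a random listed prop via physics impulses, and a threshold check gates random light and front-door events.
; Sounds and EMF level updates accompany the disturbances.
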(event OnComponentBeginOverlap(Box)
  (params (OverlappedComponent :type Primitive%20Component%20Object%20Reference) (OtherActor :type Actor%20Object%20Reference) (OtherComp :type Primitive%20Component%20Object%20Reference) (OtherBodyIndex :type Integer) (bFromSweep :type Boolean) (SweepResult :type Hit%20Result%20Structure%20%28by%20ref%29))
  ;[1 1 1] Begin Overlap
  (Utilities|Casting|CastToGhostophobiaCharacter OtherActor)
  (Variables|Default|SetIn%20Home true)
  (CallFunction|GetVarinHome)
  (bind _returnvalue (Utilities|Time|SetTimerbyEvent (delegate Custom|Ghost%20Events) (Variables|Default|GetTime) true))
  (Variables|Default|SetTimer _returnvalue))

(event OnComponentEndOverlap(Box)
  (params (OverlappedComponent :type Primitive%20Component%20Object%20Reference) (OtherActor :type Actor%20Object%20Reference) (OtherComp :type Primitive%20Component%20Object%20Reference) (OtherBodyIndex :type Integer))
  (bind _timer (Variables|Default|GetTimer))
  ;[1 1 1] End Overlap
  (Utilities|Casting|CastToGhostophobiaCharacter OtherActor)
  (Variables|Default|SetIn%20Home false)
  (CallFunction|GetVarinHome)
  (Utilities|Time|PauseTimerbyHandle _timer)
  (Utilities|Time|ClearandInvalidateTimerbyHandle _timer)
  (Class|Ghostophobia|UpdateEmfLevel(Message) (Variables|Default|GetEMF) 1))

(event Custom|Ghost%20Events
  (bind _timer (Variables|Default|GetTimer))
  (CallFunction|KickActor)
  (Utilities|FlowControl|Delay 0.2)
  (Class|Ghostophobia|UpdateEmfLevel(Message) (Variables|Default|GetEMF) 1)
  (if (Utilities|Time|IsTimerActivebyHandle _timer)
    (if (>= (Class|KismetSystemLibrary|GetTimerElapsedTimeHandle _timer) (Variables|Default|GetActivity%20Timer))
      (CallFunction|TurnOffAllLights (Variables|Default|GetAll%20Lamp))
      (CallFunction|InteractDoorGhost))))

(event Custom|Turn%20Off%20All%20Lights
  (params (Array :type Array%20of%20BP%20Lamp%2003%20ON%20Object%20References))
  ;[1 1 1] Ghost Event | Turn Off All Lights
  (CallFunction|TurnOff Array))

(event Custom|Turn%20Off
  (params (Array :type Array%20of%20BP%20Lamp%2003%20ON%20Object%20References))
  ;[1 1 1] Ghost Event | Turn Off All Lights
  (for _array_element Array
    (Default|DisableLight _array_element (Math|Random|RandomBool) (Transformation|GetActorLocation _array_element))))

(event Custom|Interact%20All%20Door%20Front
  ;[1 1 1] Ghost Event | Door
  (Utilities|Random
    (:True
      (for _array_element (Variables|Default|GetDoor%20Front)
        (Default|MoveDoor _array_element)
        (CallFunction|PlaySound "/Game/GhostophobiaBP/Audio/SoundCue/Door_Ghost.Door_Ghost" (Transformation|GetActorLocation _array_element) "/Game/GhostophobiaBP/Audio/Attenuation/Voip_Walk_Small_Distance.Voip_Walk_Small_Distance")
        (Class|Ghostophobia|UpdateEmfLevel(Message) (Variables|Default|GetEMF) 5)))))

(event Custom|Interact%20Random%20Door%20%28front%29
  (bind _outitem (CallFunction|GetRandomDoorFront))
  ;[1 1 1] Ghost Event | Door
  (Utilities|Random
    (:False
      (Utilities|Random
        (:True
          (Default|MoveDoor _outitem)
          (CallFunction|PlaySound "/Game/GhostophobiaBP/Audio/SoundCue/Door_Ghost.Door_Ghost" (Transformation|GetActorLocation _outitem) "/Game/GhostophobiaBP/Audio/Attenuation/Voip_Walk_Small_Distance.Voip_Walk_Small_Distance")
          (Class|Ghostophobia|UpdateEmfLevel(Message) (Variables|Default|GetEMF) 5))))))

(event Custom|Interact%20All%20Door%20Interior
  ;[1 1 1] Ghost Event | Door
  (Utilities|Random
    (:False
      (for _array_element (Variables|Default|GetDoor%20Interior)
        (Default|MoveDoorServer _array_element)
        (CallFunction|PlaySound "/Game/GhostophobiaBP/Audio/SoundCue/Door_Ghost.Door_Ghost" (Transformation|GetActorLocation _array_element) "/Game/GhostophobiaBP/Audio/Attenuation/Voip_Walk_Small_Distance.Voip_Walk_Small_Distance")))))

(event Custom|Interact%20Door%20ghost
  ;[1 1 1] Ghost Event | Door
  (Utilities|Random
    (:True
      (CallFunction|InteractAllDoorFront))
    (:False
      (CallFunction|InteractRandomDoor(front)))))

(event Custom|Interact%20Random%20Door%20Interior
  (bind _outitem (CallFunction|GetRandomDoorInterior))
  ;[1 1 1] Ghost Event | Door
  (Utilities|Random
    (:True
      (Utilities|Random
        (:True
          (Default|MoveDoorServer _outitem)
          (CallFunction|PlaySound "/Game/GhostophobiaBP/Audio/SoundCue/Door_Ghost.Door_Ghost" (Transformation|GetActorLocation _outitem) "/Game/GhostophobiaBP/Audio/Attenuation/Voip_Walk_Small_Distance.Voip_Walk_Small_Distance"))))))

(event Custom|Play%20Sound
  (params (Sound :type Sound%20Base%20Object%20Reference) (Location :type Vector) (AttenuationSettings :type Sound%20Attenuation%20Object%20Reference))
  (CallFunction|PlaySoundDoorClient Location Sound AttenuationSettings))

(event Custom|Play%20Sound%20Door%20Client
  (params (Location :type Vector) (Sound :type Sound%20Base%20Object%20Reference) (AttenuationSettings :type Sound%20Attenuation%20Object%20Reference))
  (Audio|PlaySoundatLocation Sound Location "0, 0, 0" 1.0 1.0 0.0 AttenuationSettings 0 0))

(event EventBeginPlay
  ;[1 1 1] Begin Play
  (Variables|Default|SetController (.AsGhostophobia%20Controller (Utilities|Casting|CastToGhostophobiaController (Game|GetPlayerController 0))))
  (Networking|SwitchHasAuthority
    (:Authority
      (Default|SetGhostType (Variables|Default|GetGhost)))))

(fn ConstructionScript
  (switch Utilities|FlowControl|Switch|SwitchonGhostType (Variables|/Game/GhostophobiaBP/Blueprints/Ghost/Ghost.Ghost_C|GetE_Ghost (Variables|Default|GetGhost))
    (:NewEnumerator0
      (Variables|Default|SetTime 15.0)
      (Variables|Default|SetActivity%20Timer 1e+01))
    (:NewEnumerator1
      (Variables|Default|SetTime 1e+01)
      (Variables|Default|SetActivity%20Timer 5.0))
    (:NewEnumerator2
      (Variables|Default|SetTime 1e+01)
      (Variables|Default|SetActivity%20Timer 4.0))))

(fn GetVarinHome
  (Development|PrintString (Utilities|String|ToString(Boolean) (Variables|Default|GetIn%20Home))))

(fn GetRandomActorfromList
  (return (.OutItem (Utilities|Array|Random (Variables|Default|GetActor%20List)))))

(fn KickActor
  ;[1 1 1] Проверяется игрок дома или нет
  (if (Variables|Default|GetIn%20Home)
    ;[1 1 1] Из массива рандомно берётся актор
    (bind _output_get (Variables|Default|SetSelecteed (CallFunction|GetRandomActorfromList)))
    ;[1 1 1 1 12] Тут идёт определения по типам
    (switch Utilities|FlowControl|Switch|SwitchonGhostType (Variables|/Game/GhostophobiaBP/Blueprints/Ghost/Ghost.Ghost_C|GetE_Ghost (Variables|Default|GetGhost))
      (:NewEnumerator0
        (Utilities|Random
          (:True
            _)))
      (:NewEnumerator1
        (Utilities|Random
          (:False
            (Utilities|Random
              (:True
                _)))))
      (:NewEnumerator2
        _))
    (Utilities|IsSimulatePhysic? _output_get
      (:True
        (CallFunction|AddImpulse (Variables|Default|GetSelecteed)))
      (:False
        (CallFunction|SimulatePhysic (Variables|Default|GetSelecteed) true)
        (CallFunction|AddImpulse (Variables|Default|GetSelecteed))))
    (CallFunction|SimulatePhysic (Variables|Default|GetSelecteed) false)
    (CallFunction|SetEMFLevel 5)
    (Variables|Default|SetSelecteed 0)
    (return true (Variables|Default|GetSelecteed) 0)))

(fn SimulatePhysic
  (params (NewParam :type Static%20Mesh%20Actor%20Object%20Reference) (bSimulate :type Boolean))
  (Physics|SetSimulatePhysics (Variables|/Script/Engine.StaticMeshActor|GetStaticMeshComponent NewParam) bSimulate)
  (return bSimulate))

(fn AddImpulse
  (params (For%20Impulse :type Static%20Mesh%20Actor%20Object%20Reference))
  (bind _returnvalue (Math|Random|RandomFloatinRange 1e+02 1.5e+02))
  (Physics|AddImpulse (Variables|/Script/Engine.StaticMeshActor|GetStaticMeshComponent For%20Impulse) (Math|Vector|MakeVector 0.0 0.0 _returnvalue) "None" false)
  (Class|PrimitiveComponent|AddAngularImpulseinRadians (Variables|/Script/Engine.StaticMeshActor|GetStaticMeshComponent For%20Impulse) (Math|Conversions|ToVector(Float) _returnvalue) "None" true)
  (Audio|PlaySoundatLocation "/Game/GhostophobiaBP/Audio/SoundCue/Throwing.Throwing" (Transformation|GetActorLocation For%20Impulse) "0, 0, 0" 1.0 1.0 0.0 "/Game/GhostophobiaBP/Audio/Attenuation/Voip_Walk_Small_Distance.Voip_Walk_Small_Distance" 0 0)
  (return true))

(fn GetRandomDoorFront
  (return (.OutItem (Utilities|Array|Random (Variables|Default|GetDoor%20Front)))))

(fn GetRandomDoorInterior
  (return (.OutItem (Utilities|Array|Random (Variables|Default|GetDoor%20Interior)))))

(fn SetEMFLevel
  (params (Emf :type Byte))
  (bind _output_get (Variables|/Game/GhostophobiaBP/Blueprints/Ghost/Ghost.Ghost_C|SetEmf (Variables|Default|GetGhost) Emf))
  (Class|Ghostophobia|UpdateEmfLevel(Message) (Variables|Default|GetEMF) (Math|Conversions|ToInteger(Byte) _output_get))
  (return true _output_get))