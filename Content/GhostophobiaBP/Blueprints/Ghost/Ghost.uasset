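; Ghost Blueprint that holds a ghost type and picks it at random for the game.
; SetGhostType converts a random byte from a limited range into the ghost enum and prints the result for debugging.
; Switch On Ghost branches execution by type: Ghost, Poltergeist, Demon or None.
; A Data Table helper looks up a row and switches on its ghost type, but that switch is unconnected and its return never runs.
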(event Custom|Set%20Ghost%20Type
  (bind _output_get (Variables|Default|SetE_Ghost (Utilities|Enum|ByteToEnumGhostType (CallFunction|RandomByteinRange 1 2))))
  (Development|PrintString (Utilities|String|EnumtoString _output_get)))

(fn DataTable
  (params (DataTable :type Data%20Table%20Object%20Reference) (RowName :type Name))
  (bind _returnvalue (Utilities|GetDataTableRow DataTable RowName)
    (:then
      (switch Utilities|FlowControl|Switch|SwitchonGhostType (.TypeGhost (Utilities|Struct|BreakGhostSt _returnvalue))))))