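; Lobby player controller that manages each player's info and lobby menu.
; It creates the lobby widget with a visible cursor and rebuilds its player list whenever connected-player data is passed in.
; Initialization and nickname changes, routed through server- and client-named events, store the player info struct and ask LobbyGM to update everyone.
; End play calls widget removal.
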(event Custom|Initialize%20Setup
  ;[1 1 1] Initialization
  (CallFunction|CallUpdate (Variables|Default|GetPlayerInfo)))

(event Custom|Remove%20all%20widgets
  (params (Widget :type User%20Widget%20Object%20Reference))
  (Widget|RemovefromParent Widget))

(event Custom|Call%20Update
  (params (NewParam :type Info%20Game%20Structure))
  ;[1 1 1] Call Update
  (Variables|Default|SetPlayerInfo NewParam)
  (bind _aslobby_gm (Utilities|Casting|CastToLobbyGM (Game|GetGameMode)))
  (Default|EveryoneUpdate _aslobby_gm))

(event Custom|Setup%20Lobby%20Widget
  ;[1 1 1] Setup Lobby Widget
  (Variables|Default|SetbShowMouseCursor true)
  (bind _returnvalue (UserInterface|CreateWidget "/Game/GhostophobiaBP/Widgets/LobbyWindow.LobbyWindow_C"))
  (bind _output_get (Variables|Default|SetLobbyMenu _returnvalue))
  (UserInterface|Viewport|AddtoViewport _output_get 0))

(event Custom|Add%20Player%20Info
  (params (Connected%20Players :type Array%20of%20Info%20Game%20Structures))
  (bind _lobbymenu (Variables|Default|GetLobbyMenu))
  ;[1 1 1] Add player info
  (bind _output_get (Variables|Default|SetConnected%20Players Connected%20Players))
  (Utilities|IsValid _lobbymenu
    (:Is%20Valid
      (Default|ClearList _lobbymenu)
      (for _array_element _output_get
        (Default|UpdatePlayerList _lobbymenu _array_element)))))

(event Custom|Set%20Nickname%20Server
  (params (Nick :type Text))
  (CallFunction|SetNicknameClient Nick))

(event Custom|Set%20Nickname%20Client
  (params (Nick :type Text))
  (bind _structout (CallFunction|SetNickname Nick))
  (CallFunction|CallUpdate _structout))

(event EventEndPlay
  (params (EndPlayReason :type EEndPlayReason%20Enum :default "Destroyed"))
  ;[1 1 1] End Play
  (Viewport|RemoveAllWidgets))

(fn ConstructionScript)

(fn SetNickname
  (params (Nick :type Text))
  (bind _structout (Utilities|Struct|SetmembersinInfoGame (Variables|Default|GetPlayerInfo) Nick))
  (return _structout))