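; Weapon Blueprint for Ghostophobia that decides whether the player can take a weapon.
; On BeginPlay it caches the player character as a GhostophobiaCharacter.
; CheckAndTakeWeapon stores the passed EWeapon value and returns true only if that character has no weapon, actor or video camera.
; The CheckAndTakeWeap event wraps this function but ignores its result, and nothing here attaches the weapon or updates the character.
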(event Custom|Check%20And%20Take%20Weap
  (params (E_Weapon :type Weapon%20Enum :default "NewEnumerator0"))
  (CallFunction|CheckandTakeWeapon E_Weapon))

(event EventBeginPlay
  (bind _asghostophobia_character (Utilities|Casting|CastToGhostophobiaCharacter (Game|GetPlayerCharacter 0)))
  (Variables|Default|SetChar _asghostophobia_character))

(fn CheckandTakeWeapon
  (params (E_Weapon :type Weapon%20Enum :default "NewEnumerator0"))
  (bind _char (Variables|Default|GetChar))
  (if (not (Variables|/Game/GhostophobiaBP/Character/Blueprints/GhostophobiaCharacter.GhostophobiaCharacter_C|GetHave%20Weapon _char))
    (if (not (Variables|/Game/GhostophobiaBP/Character/Blueprints/GhostophobiaCharacter.GhostophobiaCharacter_C|GetHave%20Actor _char))
      (if (not (Variables|/Game/GhostophobiaBP/Character/Blueprints/GhostophobiaCharacter.GhostophobiaCharacter_C|GetHave%20Video%20Camera _char))
        (Variables|Default|SetE_Weapon E_Weapon)
        (return true)))))