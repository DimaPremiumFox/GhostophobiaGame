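; Player controller for Ghostophobia that handles the journal book UI and push-to-talk voice chat.
; Pressing H alternates between creating a new Book widget with the mouse cursor shown and removing it with the cursor hidden.
; Holding V starts networked voice transmission, and releasing it stops it.
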(event Input|KeyboardEvents|V
  (params (Key :type Key%20Structure :default "None"))
  (:Pressed
    (Class|AdvancedVoiceLibrary|StartNetworkedVoice))
  (:Released
    (Class|AdvancedVoiceLibrary|StopNetworkedVoice)))

(event Input|KeyboardEvents|H
  (params (Key :type Key%20Structure :default "None"))
  (:Pressed
    (Utilities|FlowControl|FlipFlop
      (:A
        (bind _returnvalue (UserInterface|CreateWidget "/Game/GhostophobiaBP/Widgets/Book.Book_C"))
        (bind _output_get (Variables|Default|SetBook _returnvalue))
        (UserInterface|Viewport|AddtoViewport _output_get 0)
        (CallFunction|SetShowMouseCursor true))
      (:B
        (bind _book (Variables|Default|GetBook)
          (:then
            (Widget|RemovefromParent _book)
            (CallFunction|SetShowMouseCursor false))
          (:else))))))

(fn ConstructionScript)