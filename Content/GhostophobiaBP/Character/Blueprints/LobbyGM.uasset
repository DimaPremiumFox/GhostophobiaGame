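; Lobby game mode that tracks connected players and moves the session to Tanglewood_Street once all are ready.
; PostLogin registers controllers on the server and sets up their lobby widgets, while OnLogout removes them.
; Both then trigger EveryoneUpdate, which rebuilds the player info list and pushes it to every LobbyController.
; The ready check stops at the first unready player, otherwise LaunchLobby issues a servertravel console command after a short delay.
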(event Custom|Everyone%20Update
  (bind _all_player_controllers (Variables|Default|GetAll%20Player%20Controllers))
  ;[1 1 1] Everyone Update
  (Variables|Default|SetCurrent%20Connections (Utilities|Array|Length (Variables|Default|GetAll%20Player%20Controllers)))
  (Utilities|Array|Clear (Variables|Default|GetConnected%20Players%20Info))
  (for _array_element _all_player_controllers
    (bind _aslobby_controller (Utilities|Casting|CastToLobbyController _array_element))
    (Utilities|Array|Add (Variables|Default|GetConnected%20Players%20Info) (Variables|/Game/GhostophobiaBP/Character/Blueprints/LobbyController.LobbyController_C|GetPlayerInfo _aslobby_controller)))
  (for _array_element_2 _all_player_controllers
    (bind _aslobby_controller_2 (Utilities|Casting|CastToLobbyController _array_element_2))
    (Default|AddPlayerInfo _aslobby_controller_2 (Variables|Default|GetConnected%20Players%20Info))))

(event Custom|Check%20players%20%28Ready%29
  ;[1 1 1] Check players if they are ready
  (bind _array_element (Utilities|Array|ForEachLoopwithBreak (Variables|Default|GetConnected%20Players%20Info))
    (:LoopBody
      (if (Utilities|Struct|BreakInfoGame _array_element)
        (Variables|Default|SetCanStartGame true)
        (else
          (Variables|Default|SetCanStartGame false)
          (CallFunction|CannotStartGame))))
    (:Completed
      (CallFunction|LaunchLobby))))

(event Custom|Cannot%20Start%20Game
  ;[1 1 1] Check players if they are ready
  (Utilities|Array|ForEachLoopwithBreak (Variables|Default|GetConnected%20Players%20Info)) ; enters at Break
)

(event Custom|Launch%20Session
  (params (B :type String))
  ;[1 1 1] Launch Session
  (Development|ExecuteConsoleCommand (Utilities|String|Append "servertravel " B) (Game|GetPlayerController 0)))

(event Custom|Travel%20To
  (params (Mapname :type String))
  (Development|ExecuteConsoleCommand (Utilities|String|Append "Servertravel " Mapname) (Game|GetPlayerController 0)))

(event Custom|Launch%20Lobby
  ;[1 1 1] Launch Lobby
  (if (Variables|Default|GetCanStartGame)
    (Utilities|FlowControl|Delay 0.2)
    (CallFunction|Travelto "Tanglewood_Street")))

(event EventPostLogin
  (params (NewPlayer :type Player%20Controller%20Object%20Reference))
  ;[1 1 1] Post Login
  (Networking|SwitchHasAuthority
    (:Authority
      (Utilities|Array|Add (Variables|Default|GetAll%20Player%20Controllers) NewPlayer)
      (bind _aslobby_controller (Utilities|Casting|CastToLobbyController NewPlayer))
      (bind _output_get (Variables|Default|SetLC _aslobby_controller))
      (Default|InitializeSetup _output_get)
      (Default|SetupLobbyWidget _output_get)
      (CallFunction|EveryoneUpdate))))

(event EventOnLogout
  (params (ExitingController :type Controller%20Object%20Reference))
  (bind _all_player_controllers (Variables|Default|GetAll%20Player%20Controllers))
  ;[1 1 1] Event OnLogout - End Event
  (bind (_array_element _array_index) (Utilities|Array|ForEachLoopwithBreak _all_player_controllers :!label _label)
    (:LoopBody
      (if (== _array_element ExitingController)
        (goto _label Break)))
    (:Completed
      (Utilities|Array|RemoveIndex _all_player_controllers _array_index)
      (Utilities|Array|RemoveIndex (Variables|Default|GetConnected%20Players%20Info) _array_index)
      (CallFunction|EveryoneUpdate))))

(fn ConstructionScript)

(fn GetTravelCommand
  (params (B :type String))
  (return (Utilities|String|Append "servertravel" B)))