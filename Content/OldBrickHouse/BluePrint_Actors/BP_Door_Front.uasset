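; Front door actor for the old brick house that the player character opens and closes through interaction.
; Interact accepts only a GhostophobiaCharacter, then calls MoveDoor and MoveDoorCl, which plays or reverses a timeline based on its current value.
; The timeline drives the door mesh's yaw, with IsOpeningInwards selecting the direction.
; Target events forward to a child-actor widget, configured by override functions with a "Door" title and Interact key bind.
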(event Custom|MoveDoor
  (CallFunction|MoveDoorCl))

(event Custom|Move%20Door%20Cl
  (bind _sm_door_front (Variables|Default|GetSM_Door_Front))
  (if (< (stale _axisz) 1.0)
    (bind _axisz (Timeline|Timeline_0 Play)
      (:Update
        (if (Variables|Default|GetisOpeningInwards)
          (Transformation|SetRelativeRotation _sm_door_front (Math|Rotator|MakeRotator 0.0 0.0 _axisz) false false)
          (else
            (Transformation|SetRelativeRotation _sm_door_front (Math|Rotator|MakeRotator 0.0 0.0 (- 1.0 _axisz)) false false)))))
    (else
      (Timeline|Timeline_0 Reverse))))

(event EventInteract
  (params (Key :type Key%20Structure) (Pawn :type Pawn%20Object%20Reference))
  (Utilities|Casting|CastToGhostophobiaCharacter Pawn)
  (CallFunction|MoveDoor))

(event EventCurrentTarget
  (params (Pawn :type Pawn%20Object%20Reference))
  (bind _widget (Variables|Default|GetWidget))
  (bind _childactor (Variables|/Script/Engine.ChildActorComponent|GetChildActor _widget))
  ;[1 1 1] Current target (Copy and paste this in to your own actor)
  (Class|InteractionInterface|CurrentTarget(Message) _childactor Pawn)
  (Class|InteractionInterface|ParentActor(Message) _childactor self))

(event EventClearTarget
  ;[1 1 1] Clear target (Copy and paste this in to your own actor)
  (Class|InteractionInterface|ClearTarget(Message) (Variables|/Script/Engine.ChildActorComponent|GetChildActor (Variables|Default|GetWidget))))

(fn ConstructionScript)

(fn SetDetail1
  (return false ""))

(fn SetDetail2
  (return false ""))

(fn SetDetail3
  (return false ""))

(fn SetDetail4
  (return false ""))

(fn SetWidgetAmount
  (return false 0))

(fn SetWidgetColor
  (return "" ""))

(fn SetWidgetKeyBinds
  (return true (Utilities|Array|MakeArray (Utilities|Struct|MakeS_KeyBinds "E" "Interact"))))

(fn SetWidgetLevel
  (return false ""))

(fn SetWidgetSubTitle
  (return false ""))

(fn SetWidgetTitle
  (return true "Door"))

(fn SetWidgetType
  (return "NewEnumerator1"))